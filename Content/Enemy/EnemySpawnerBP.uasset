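; Enemy spawner actor that creates escalating waves of EnemyAI at its own location.
; On BeginPlay it binds SpawnEnemy to the wave spawn event of BP_ThirdPersonGameMode, so the game mode drives wave timing.
; Each wave spawns the current enemy count at the spawner's transform, then raises an increment and adds it to the count, so each wave grows by a larger step.
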(event Custom|SpawnEnemy
  (for _index (range 0 (- (Variables|Default|GetEnemySpawned) 1))
    (Game|SpawnActorfromClass "/Game/Enemy/EnemyAI.EnemyAI_C" (Transformation|GetActorTransform) "Undefined" 0 0))
  (Math|Integer|IncrementInt (Variables|Default|GetSpawnIncrement)
    (:%20%20
      (Variables|Default|SetEnemySpawned (+ (Variables|Default|GetEnemySpawned) (Variables|Default|GetSpawnIncrement))))))

(event EventBeginPlay
  (bind _asbp_third_person_game_mode (Utilities|Casting|CastToBP_ThirdPersonGameMode (Game|GetGameMode)))
  (EventDispatchers|BindEventtoWaveSpawn _asbp_third_person_game_mode (delegate Custom|SpawnEnemy)))

(fn ConstructionScript)